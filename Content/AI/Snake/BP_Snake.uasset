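; Snake AI character that patrols, reacts to the player and bites on contact.
; Unless nomadic, it gathers nearby patrol nodes on BeginPlay.
; Perception sets Neutral, Aware or Threatened by player distance, with delayed reset; the RepNotify pushes AlertState to the Blackboard and adjusts walk speed.
; Overlap triggers a gated attack that slows the snake, applies randomized damage and repeats after the montage while the player remains inside its box.
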(event OnTargetPerceptionUpdated(AIPerception)
  (params (Actor :type Actor%20Object%20Reference) (Stimulus :type AI%20Stimulus%20Structure))
  (if (and (.bSuccessfullySensed (Utilities|Struct|BreakAIStimulus Stimulus)) (== Actor (Game|Player|GetPlayerPawn 0)))
    (Variables|Default|SetAlertState (select (<= (Math|Vector|Distance(Vector) (Transformation|GetActorLocation) (Transformation|GetActorLocation Actor)) 5e+02) "NewEnumerator2" "NewEnumerator1"))
    (Utilities|FlowControl|Sequence
      (:then_0
        (if (Utilities|Enum|NotEqual(Enum) (Variables|Default|GetAlertState) "NewEnumerator0")
          (Utilities|FlowControl|Delay 0.2)
          (Variables|Default|SetAlertState (select (<= (Math|Vector|Distance(Vector) (Transformation|GetActorLocation) (Transformation|GetActorLocation (Game|Player|GetPlayerPawn 0))) 5e+02) "NewEnumerator2" "NewEnumerator1"))))
      (:then_1
        (Utilities|FlowControl|DoOnce false :!label _label
          (:Completed
            (Audio|PlaySound2D "/Game/AI/Temp_Alert_Sound.Temp_Alert_Sound" 1.0 1.0 0.0 0 0))))
      (:then_2
        (Utilities|FlowControl|Delay 1.0)
        (goto _label Reset)))
    (else
      (Utilities|FlowControl|RetriggerableDelay 5.0)
      (Variables|Default|SetAlertState "NewEnumerator0"))))

(event EventBeginPlay
  (Default|ResetAI (.AsSnake%20AIController%20BP (Utilities|Casting|CastToSnakeAIController_BP (Pawn|GetController))))
  (if (not (Variables|Default|GetIsNomadic?))
    (bind _outactors (Actor|GetAllActorsOfClass "/Game/AI/Snake/SnakePatrolNode.SnakePatrolNode_C"))
    (for _array_element _outactors
      (if (<= (Math|Vector|Distance(Vector) (Transformation|GetActorLocation) (Transformation|GetActorLocation _array_element)) 2.5e+03)
        (Utilities|Array|AddUnique (Variables|Default|GetPatrolNodeArray) _array_element)))))

(event Collision|EventActorBeginOverlap
  (params (OtherActor :type Actor%20Object%20Reference))
  (bind _damage (Variables|Default|GetDamage))
  (bind _asals_anim_man_character_bp (Utilities|Casting|CastToALS_AnimMan_CharacterBP OtherActor))
  (Utilities|FlowControl|Gate false :!label _label
    (:Exit
      (Variables|Default|SetAttacking true)
      (Variables|/Script/Engine.CharacterMovementComponent|SetMaxWalkSpeed (Variables|Character|GetCharacterMovement) 3e+01)
      (Utilities|FlowControl|Sequence
        (:then_0
          (Development|PrintString "CONTACTEDPLAYER")
          (bind _returnvalue (Animation|PlayAnimMontage "/Game/AdvancedLocomotionV4/CharacterAssets/MannequinSkeleton/AnimationExamples/Actions/ALS_CLF_GetUp_Back_Montage_2H.ALS_CLF_GetUp_Back_Montage_2H" 1.0 "None"))
          (Game|Damage|ApplyDamage _asals_anim_man_character_bp (Math|Random|RandomFloatinRange (- _damage 3.0) (+ _damage 4.0)) 0 0)
          (Utilities|FlowControl|Delay _returnvalue)
          (Variables|Default|SetAttacking false))
        (:then_1
          (goto _label Close))
        (:then_2
          (Utilities|FlowControl|Delay _returnvalue)
          (Utilities|FlowControl|Sequence
            (:then_0
              (goto _label Open))
            (:then_1
              (if (Collision|IsOverlappingActor (Variables|Default|GetBox) (Game|Player|GetPlayerPawn 0) :!class /Script/Engine.PrimitiveComponent)
                (goto _label)))))))))

(event EventTick
  (params (DeltaSeconds :type Float%20%28single-precision%29))
  (Development|PrintString (Utilities|String|EnumtoString (Variables|Default|GetAlertState)) true true "(R=0.000000,G=0.660000,B=1.000000,A=1.000000)" DeltaSeconds))

(fn ConstructionScript)

(fn OnRepAlertState
  (bind _alertstate (Variables|Default|GetAlertState))
  (AI|Components|Blackboard|SetValueasEnum (AI|GetBlackboard (Pawn|GetController)) (Utilities|Name|MakeLiteralName "AlertState") _alertstate)
  (Variables|/Script/Engine.CharacterMovementComponent|SetMaxWalkSpeed (Variables|Character|GetCharacterMovement) (Utilities|Select :Index _alertstate :NewEnumerator0 2e+02 :NewEnumerator1 3e+02 :NewEnumerator2 4.5e+02)))