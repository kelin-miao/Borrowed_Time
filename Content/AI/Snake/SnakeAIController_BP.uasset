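; AI controller for the snake enemy that starts its behavior tree and seeds the blackboard.
; On BeginPlay it runs SnakeAI_BT, then copies the possessed BP_Snake's nomadic flag and the first player's pawn into the IsNomad and PlayerPawn keys.
; A ResetAI event re-enters the same setup sequence, so the tree run and blackboard values can be reapplied after startup.
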(event Custom|ResetAI
  (bind _blackboard (Variables|Default|GetBlackboard))
  (AI|RunBehaviorTree "/Game/AI/Snake/SnakeAI_BT.SnakeAI_BT")
  (bind _asbp_snake (Utilities|Casting|CastToBP_Snake (Pawn|GetControlledPawn)))
  (AI|Components|Blackboard|SetValueasBool _blackboard (Utilities|Name|MakeLiteralName "IsNomad") (Variables|/Game/AI/Snake/BP_Snake.BP_Snake_C|GetIsNomadic? _asbp_snake))
  (AI|Components|Blackboard|SetValueasObject _blackboard (Utilities|Name|MakeLiteralName "PlayerPawn") (Game|Player|GetPlayerPawn 0)))

(event EventBeginPlay
  (bind _blackboard (Variables|Default|GetBlackboard))
  (AI|RunBehaviorTree "/Game/AI/Snake/SnakeAI_BT.SnakeAI_BT")
  (bind _asbp_snake (Utilities|Casting|CastToBP_Snake (Pawn|GetControlledPawn)))
  (AI|Components|Blackboard|SetValueasBool _blackboard (Utilities|Name|MakeLiteralName "IsNomad") (Variables|/Game/AI/Snake/BP_Snake.BP_Snake_C|GetIsNomadic? _asbp_snake))
  (AI|Components|Blackboard|SetValueasObject _blackboard (Utilities|Name|MakeLiteralName "PlayerPawn") (Game|Player|GetPlayerPawn 0)))

(event EventTick
  (params (DeltaSeconds :type Float%20%28single-precision%29)))

(fn ConstructionScript)