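; Bear AI character that patrols and reacts to the player through Neutral, Aware and Threatened alert states.
; Non-nomadic bears collect nearby BearPatrolNodes at BeginPlay.
; AI Perception sets the state by player distance, rechecks shortly after, plays a throttled alert sound, and reverts to Neutral through a retriggerable delay.
; AlertState's RepNotify feeds the Blackboard and scales walk speed; Tick prints the state for debugging.
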(event OnTargetPerceptionUpdated(AIPerception)
  (params (Actor :type Actor%20Object%20Reference) (Stimulus :type AI%20Stimulus%20Structure))
  (if (and (.bSuccessfullySensed (Utilities|Struct|BreakAIStimulus Stimulus)) (== Actor (Game|Player|GetPlayerPawn 0)))
    (Variables|Default|SetAlertState (select (<= (Math|Vector|Distance(Vector) (Transformation|GetActorLocation) (Transformation|GetActorLocation Actor)) 5e+02) "NewEnumerator2" "NewEnumerator1"))
    (Utilities|FlowControl|Sequence
      (:then_0
        (if (Utilities|Enum|NotEqual(Enum) (Variables|Default|GetAlertState) "NewEnumerator0")
          (Utilities|FlowControl|Delay 0.2)
          (Variables|Default|SetAlertState (select (<= (Math|Vector|Distance(Vector) (Transformation|GetActorLocation) (Transformation|GetActorLocation (Game|Player|GetPlayerPawn 0))) 5e+02) "NewEnumerator2" "NewEnumerator1"))))
      (:then_1
        (Utilities|FlowControl|DoOnce false :!label _label
          (:Completed
            (Audio|PlaySound2D "/Game/AI/Bear/Temp_Alert_Sound.Temp_Alert_Sound" 1.0 1.0 0.0 0 0))))
      (:then_2
        (Utilities|FlowControl|Delay 1.0)
        (goto _label Reset)))
    (else
      (Utilities|FlowControl|RetriggerableDelay 5.0)
      (Variables|Default|SetAlertState "NewEnumerator0"))))

(event EventBeginPlay
  (if (not (Variables|Default|GetIsNomadic?))
    (bind _outactors (Actor|GetAllActorsOfClass "/Game/AI/Bear/BearPatrolNode.BearPatrolNode_C"))
    (for _array_element _outactors
      (if (<= (Math|Vector|Distance(Vector) (Transformation|GetActorLocation) (Transformation|GetActorLocation _array_element)) 2.5e+03)
        (Utilities|Array|AddUnique (Variables|Default|GetPatrolNodeArray) _array_element)))))

(event Collision|EventActorBeginOverlap
  (params (OtherActor :type Actor%20Object%20Reference)))

(event EventTick
  (params (DeltaSeconds :type Float%20%28single-precision%29))
  (Development|PrintString (Utilities|String|EnumtoString (Variables|Default|GetAlertState)) true true "(R=0.000000,G=0.660000,B=1.000000,A=1.000000)" DeltaSeconds))

(fn ConstructionScript)

(fn OnRepAlertState
  (bind _alertstate (Variables|Default|GetAlertState))
  (AI|Components|Blackboard|SetValueasEnum (AI|GetBlackboard (Pawn|GetController)) (Utilities|Name|MakeLiteralName "AlertState") _alertstate)
  (Variables|/Script/Engine.CharacterMovementComponent|SetMaxWalkSpeed (Variables|Character|GetCharacterMovement) (Utilities|Select :Index _alertstate :NewEnumerator0 2e+02 :NewEnumerator1 3e+02 :NewEnumerator2 4.5e+02)))