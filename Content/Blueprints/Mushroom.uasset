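; Foraging mushroom actor that the player eats on interaction, either edible for nourishment or poisonous for damage.
; The construction script randomly picks the variant (reusing the BerryBushTypes enum) and a matching mesh, then a delayed BeginPlay sets its nutrition and health effect.
; Interact applies both effects to the ALS character, then hides the mesh and ignores its trace channel rather than destroying the actor.
; A debug text label shows the variant and turns toward the player.
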(event Custom|Randomise
  (bind _poisonous_mushroom_meshes (Variables|Default|GetPoisonous%20Mushroom%20Meshes))
  (bind _edible_mushroom_meshes (Variables|Default|GetEdible%20Mushroom%20Meshes))
  (Variables|Default|SetShroom%20Variant (Utilities|Enum|ByteToEnumBerryBushTypes (Math|Conversions|ToByte(Integer) (Math|Random|RandomIntegerinRange 0 1))))
  (bind _output_get (Variables|Default|SetCurrentMesh (Utilities|Select :Index (Variables|Default|GetShroom%20Variant) :NewEnumerator0 (Utilities|Array|Get(acopy) _edible_mushroom_meshes (Math|Random|RandomIntegerinRange 0 (- (Utilities|Array|Length _edible_mushroom_meshes) 1))) :NewEnumerator1 (Utilities|Array|Get(acopy) _poisonous_mushroom_meshes (Math|Random|RandomIntegerinRange 0 (- (Utilities|Array|Length _poisonous_mushroom_meshes) 1))))))
  (Components|StaticMesh|SetStaticMesh (Variables|Default|GetStaticMesh) _output_get))

(event EventBeginPlay
  (Utilities|FlowControl|Delay 0.1)
  (CallFunction|Initialise))

(event Collision|EventActorBeginOverlap
  (params (OtherActor :type Actor%20Object%20Reference)))

(event EventTick
  (params (DeltaSeconds :type Float%20%28single-precision%29))
  (bind _berry_type_display___debug__ (Variables|Default|GetBerry%20Type%20Display%20!!DEBUG!!))
  (Utilities|FlowControl|Delay 0.2)
  (Transformation|SetRelativeRotation _berry_type_display___debug__ (Math|Rotator|FindLookatRotation (Transformation|GetWorldLocation _berry_type_display___debug__) (Transformation|GetActorLocation (Game|Player|GetPlayerPawn 0))) false false))

(event EventInteract
  (bind _asals_anim_man_character_bp (Utilities|Casting|CastToALS_AnimMan_CharacterBP (Game|Player|GetPlayerPawn 0)))
  (Variables|/Game/AdvancedLocomotionV4/Blueprints/CharacterLogic/ALS_AnimMan_CharacterBP.ALS_AnimMan_CharacterBP_C|SetNourishment _asals_anim_man_character_bp (+ (Variables|/Game/AdvancedLocomotionV4/Blueprints/CharacterLogic/ALS_AnimMan_CharacterBP.ALS_AnimMan_CharacterBP_C|GetNourishment _asals_anim_man_character_bp) (/ (Variables|Default|GetNutritional%20Value) 1e+02)))
  (Game|Damage|ApplyDamage _asals_anim_man_character_bp (* (Variables|Default|GetHealth%20Effect) -1.0) 0 0)
  (Rendering|SetVisibility (Variables|Default|GetStaticMesh) false false)
  (Collision|SetCollisionResponsetoChannel (Variables|Default|GetStaticMesh) "ECC_GameTraceChannel1" "ECR_Ignore"))

(fn ConstructionScript
  (CallFunction|Randomise))

(fn Initialise
  (Variables|Default|SetNutritional%20Value (Utilities|Select :Index (Variables|Default|GetShroom%20Variant) :NewEnumerator0 1e+01 :NewEnumerator1 0.0))
  (Variables|Default|SetHealth%20Effect (Utilities|Select :Index (Variables|Default|GetShroom%20Variant) :NewEnumerator0 0.0 :NewEnumerator1 -1e+01))
  (Rendering|Components|TextRender|SetText (Variables|Default|GetBerry%20Type%20Display%20!!DEBUG!!) (Utilities|Text|ToText(String) (Utilities|String|EnumtoString (Variables|Default|GetShroom%20Variant))))
  (Components|StaticMesh|SetStaticMesh (Variables|Default|GetStaticMesh) (Variables|Default|GetCurrentMesh)))