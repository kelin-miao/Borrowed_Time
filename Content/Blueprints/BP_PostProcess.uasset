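; Post-process actor that applies a Settings variable to its PostProcess component and drives a randomly jumping depth-of-field focus at runtime.
; The construction script copies Settings onto the component through SetSettings.
; Tick, gated by a roughly one-frame Delay, then replaces those settings with a newly built struct holding a wide aperture and a random focal distance.
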(event EventBeginPlay)

(event Collision|EventActorBeginOverlap
  (params (OtherActor :type Actor%20Object%20Reference)))

(event EventTick
  (params (DeltaSeconds :type Float%20%28single-precision%29))
  (Utilities|FlowControl|Delay 0.016)
  (Variables|/Script/Engine.PostProcessComponent|SetSettings (Variables|Default|GetPostProcess) (Utilities|Struct|MakePostProcessSettings 1.0 (Math|Random|RandomFloatinRange 0.0 1e+03))))

(fn ConstructionScript
  (CallFunction|SetSettings))

(fn SetSettings
  (Variables|/Script/Engine.PostProcessComponent|SetSettings (Variables|Default|GetPostProcess) (Variables|Default|GetSettings)))