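; Spline actor that places static meshes along its spline, alternating between two mesh choices.
; The construction script adds one Static Mesh Component per segment, positioned by lerping halfway between the local transforms of its two end points, ignoring point scale.
; A FlipFlop assigns StaticMeshA and StaticMeshB in turn.
; An unconnected spline mesh variant with forward axis and collision settings never runs, and the event graph is empty.
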(event EventBeginPlay)

(event Collision|EventActorBeginOverlap
  (params (OtherActor :type Actor%20Object%20Reference)))

(event EventTick
  (params (DeltaSeconds :type Float%20%28single-precision%29)))

(fn ConstructionScript
  (bind _spline (Variables|Default|GetSpline))
  (for _index (range 0 (- (Spline|GetNumberOfSplinePoints _spline) 2))
    (bind _returnvalue (AddComponent|AddStaticMeshComponent false (Math|Transform|Lerp(Transform) (Spline|GetTransformatSplinePoint _spline _index "Local" false) (Spline|GetTransformatSplinePoint _spline (+ _index 1) "Local" false) 0.5)))
    (Utilities|FlowControl|FlipFlop
      (:A
        (Components|StaticMesh|SetStaticMesh _returnvalue (Variables|Default|GetStatic%20Mesh%20A)))
      (:B
        (Components|StaticMesh|SetStaticMesh _returnvalue (Variables|Default|GetStatic%20Mesh%20B))))))