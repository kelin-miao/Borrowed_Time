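; BerryBush is an interactable bush whose berries change the player's nourishment and health according to their variant, from Nutritious to Toxic.
; The construction script derives nutrition and health effect from the variant, with some randomisation, and labels a debug text that periodically faces the player.
; Interact applies both effects, using negated damage for health, then swaps to a berryless mesh and ignores a trace channel.
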(event EventBeginPlay)

(event Collision|EventActorBeginOverlap
  (params (OtherActor :type Actor%20Object%20Reference)))

(event EventTick
  (params (DeltaSeconds :type Float%20%28single-precision%29))
  (bind _berry_type_display___debug__ (Variables|Default|GetBerry%20Type%20Display%20!!DEBUG!!))
  (Utilities|FlowControl|Delay 0.2)
  (Transformation|SetRelativeRotation _berry_type_display___debug__ (Math|Rotator|FindLookatRotation (Transformation|GetWorldLocation _berry_type_display___debug__) (Transformation|GetActorLocation (Game|Player|GetPlayerPawn 0))) false false))

(event EventInteract
  (bind _asals_anim_man_character_bp (Utilities|Casting|CastToALS_AnimMan_CharacterBP (Game|Player|GetPlayerPawn 0)))
  (Variables|/Game/AdvancedLocomotionV4/Blueprints/CharacterLogic/ALS_AnimMan_CharacterBP.ALS_AnimMan_CharacterBP_C|SetNourishment _asals_anim_man_character_bp (+ (Variables|/Game/AdvancedLocomotionV4/Blueprints/CharacterLogic/ALS_AnimMan_CharacterBP.ALS_AnimMan_CharacterBP_C|GetNourishment _asals_anim_man_character_bp) (/ (Variables|Default|GetNutritional%20Value) 1e+02)))
  (Game|Damage|ApplyDamage _asals_anim_man_character_bp (* (Variables|Default|GetHealth%20Effect) -1.0) 0 0)
  ;[1 1 1] No Berry Mesh
  (Components|StaticMesh|SetStaticMesh (Variables|Default|GetStaticMesh) "/Game/Tropical_Jungle_Pack/Meshes/Bush/SM_SliceBush1.SM_SliceBush1")
  (Collision|SetCollisionResponsetoChannel (Variables|Default|GetStaticMesh) "ECC_GameTraceChannel1" "ECR_Ignore"))

(fn ConstructionScript
  (bind _berry_variant (Variables|Default|GetBerry%20Variant))
  (bind _returnvalue (Utilities|Select :Index _berry_variant :NewEnumerator2 25.0 :NewEnumerator0 1e+01 :NewEnumerator3 0.0 :NewEnumerator1 -1e+01 :NewEnumerator4 -25.0))
  (Rendering|Material|SetMaterial (Variables|Default|GetStaticMesh) 0 (Utilities|Select :Index (Variables|Default|GetBerry%20Variant) :NewEnumerator2 "/Game/Tropical_Jungle_Pack/Materials/Instances/Impostor/MI_BushA_02_Impostor.MI_BushA_02_Impostor" :NewEnumerator0 "/Game/Tropical_Jungle_Pack/Materials/Instances/Impostor/MI_BushA_02_Impostor.MI_BushA_02_Impostor" :NewEnumerator3 "/Game/Tropical_Jungle_Pack/Materials/Instances/Impostor/MI_BushA_02_Impostor.MI_BushA_02_Impostor" :NewEnumerator1 "/Game/Tropical_Jungle_Pack/Materials/Instances/Impostor/MI_BushA_02_Impostor.MI_BushA_02_Impostor" :NewEnumerator4 "/Game/Tropical_Jungle_Pack/Materials/Instances/Impostor/MI_BushA_02_Impostor.MI_BushA_02_Impostor"))
  (Variables|Default|SetNutritional%20Value (Math|Random|RandomFloatinRange (- _returnvalue 5.0) (+ _returnvalue 5.0)))
  (Variables|Default|SetHealth%20Effect (Utilities|Select :Index (Variables|Default|GetBerry%20Variant) :NewEnumerator2 (Math|Random|RandomFloatinRange 3.0 7.0) :NewEnumerator0 0.0 :NewEnumerator3 0.0 :NewEnumerator1 -1e+01 :NewEnumerator4 (Math|Random|RandomFloatinRange -7.0 -3.0)))
  (Rendering|Components|TextRender|SetText (Variables|Default|GetBerry%20Type%20Display%20!!DEBUG!!) (Utilities|Text|ToText(String) (Utilities|String|EnumtoString (Variables|Default|GetBerry%20Variant)))))